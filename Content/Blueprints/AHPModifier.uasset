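; Area actor that changes a ThirdPersonCharacter's HP by a Mod amount while it stays inside a sphere.
; Sphere overlap events store the single overlapping actor and a flag, and ModHP calls itself after a one-second delay to repeat the change until overlap ends.
; The construction script tints the light component A with LightColor.
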(event OnComponentBeginOverlap(Sphere)
  (params (OverlappedComponent :type Primitive%20Component%20Object%20Reference) (OtherActor :type Actor%20Object%20Reference) (OtherComp :type Primitive%20Component%20Object%20Reference) (OtherBodyIndex :type Integer) (bFromSweep :type Boolean) (SweepResult :type Hit%20Result%20Structure%20%28by%20ref%29))
  (Variables|Default|SetOtherActor OtherActor)
  (Variables|Default|Set_isOverlapping true)
  (CallFunction|ModHP))

(event OnComponentEndOverlap(Sphere)
  (params (OverlappedComponent :type Primitive%20Component%20Object%20Reference) (OtherActor :type Actor%20Object%20Reference) (OtherComp :type Primitive%20Component%20Object%20Reference) (OtherBodyIndex :type Integer))
  (Variables|Default|SetOtherActor 0)
  (Variables|Default|Set_isOverlapping false))

(event Custom|ModHP
  (if (Variables|Default|Get_isOverlapping)
    (bind _asthird_person_character (Utilities|Casting|CastToThirdPersonCharacter (Variables|Default|GetOtherActor)))
    (Default|ModHP _asthird_person_character (Variables|Default|Get_mod))
    (Utilities|FlowControl|Delay 1.0)
    (CallFunction|ModHP)))

(event EventBeginPlay)

(event Collision|EventActorBeginOverlap
  (params (OtherActor :type Actor%20Object%20Reference)))

(event EventTick
  (params (DeltaSeconds :type Float%20%28single-precision%29)))

(fn ConstructionScript
  (Rendering|Components|Light|SetLightColor (Variables|Default|Geta) (Variables|Default|GetLightColor) true))