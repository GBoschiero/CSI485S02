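; Moving platform that slides its Cube back and forth along local X while its trigger is overlapped.
; Overlapping Animtrigger starts the PlatformAnim timeline after a short delay, and ending the overlap stops it in place.
; The timeline lerps the Cube's relative location, ping-pongs on finish, and records its direction so the next overlap resumes travel the same way.
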(event OnComponentBeginOverlap(Animtrigger)
  (params (OverlappedComponent :type Primitive%20Component%20Object%20Reference) (OtherActor :type Actor%20Object%20Reference) (OtherComp :type Primitive%20Component%20Object%20Reference) (OtherBodyIndex :type Integer) (bFromSweep :type Boolean) (SweepResult :type Hit%20Result%20Structure%20%28by%20ref%29))
  (Utilities|FlowControl|Delay 0.4)
  (CallFunction|AnimCode))

(event OnComponentEndOverlap(Animtrigger)
  (params (OverlappedComponent :type Primitive%20Component%20Object%20Reference) (OtherActor :type Actor%20Object%20Reference) (OtherComp :type Primitive%20Component%20Object%20Reference) (OtherBodyIndex :type Integer))
  (Audio|Components|Audio|Stop (Variables|Default|GetPlatformAnim)))

(event Custom|AnimCode
  (bind _platformanim (Variables|Default|GetPlatformAnim))
  (if (Utilities|Enum|Equal(Enum) (Variables|Default|Get_direction) "Forward")
    (bind (_direction _animpercedntage) (Timeline|PlatformAnim Play)
      (:Update
        (Variables|Default|Set_direction _direction)
        (Transformation|SetRelativeLocation (Variables|Default|GetCube) (Math|Vector|Lerp(Vector) "0, 0, 0" "500.000000, 0,0.000000" _animpercedntage) false false))
      (:Finished
        (if (Utilities|Enum|Equal(Enum) _direction "Forward")
          (Components|Timeline|ReversefromEnd _platformanim)
          (else
            (Components|Timeline|PlayfromStart _platformanim)))))
    (else
      (Timeline|PlatformAnim Reverse))))

(event EventBeginPlay)

(fn ConstructionScript)