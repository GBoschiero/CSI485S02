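; AMyFirstActor is a practice actor Blueprint that runs a simple win/lose check on an integer at BeginPlay.
; MyFirstFunction adds a fixed argument to the Integer variable, and BeginPlay stores and prints the sum.
; A threshold branch then prints WON or LOST.
; A disconnected chain that overrides Integer, several unused comparison nodes and an empty construction script remain in the asset.
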(event EventBeginPlay
  (bind __result (CallFunction|MyFirstFunction 15))
  (Variables|Default|Set_integer __result)
  (Development|PrintString (Utilities|String|ToString(Integer) __result))
  (if (< (Variables|Default|Get_integer) 50)
    (Development|PrintString "WON")
    (else
      (Development|PrintString "LOST"))))

(fn ConstructionScript)

(fn MyFirstFunction
  (params (_mod :type Integer))
  (return (+ _mod (Variables|Default|Get_integer))))