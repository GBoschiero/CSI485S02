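; AMagicCube is an actor whose cube doubles in size while something overlaps its box trigger.
; The construction script applies the Scale variable to the whole actor.
; Box overlap events set the Cube component's world scale to twice Scale on begin and back to Scale on end.
; Two unconnected SetActorScale3D nodes remain in the event graph and never run.
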(event OnComponentBeginOverlap(Box)
  (params (OverlappedComponent :type Primitive%20Component%20Object%20Reference) (OtherActor :type Actor%20Object%20Reference) (OtherComp :type Primitive%20Component%20Object%20Reference) (OtherBodyIndex :type Integer) (bFromSweep :type Boolean) (SweepResult :type Hit%20Result%20Structure%20%28by%20ref%29))
  (Transformation|SetWorldScale3D (Variables|Default|GetCube) (* (Variables|Default|Get_scale) 2.0)))

(event OnComponentEndOverlap(Box)
  (params (OverlappedComponent :type Primitive%20Component%20Object%20Reference) (OtherActor :type Actor%20Object%20Reference) (OtherComp :type Primitive%20Component%20Object%20Reference) (OtherBodyIndex :type Integer))
  (Transformation|SetWorldScale3D (Variables|Default|GetCube) (Variables|Default|Get_scale)))

(fn ConstructionScript
  (Transformation|SetActorScale3D (Variables|Default|Get_scale)))