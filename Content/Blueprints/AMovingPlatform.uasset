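; Moving platform actor that raises its Cube along local Z and brings it back down when something overlaps the Animtrigger component.
; The overlap waits briefly, then calls AnimCode, where the PlatformAnim timeline lerps the cube's relative location.
; On finishing, the timeline pauses and reverses, then clears IsMoving after the return trip.
; IsMoving blocks retriggers, but is only set after the initial delay.
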(event OnComponentBeginOverlap(Animtrigger)
  (params (OverlappedComponent :type Primitive%20Component%20Object%20Reference) (OtherActor :type Actor%20Object%20Reference) (OtherComp :type Primitive%20Component%20Object%20Reference) (OtherBodyIndex :type Integer) (bFromSweep :type Boolean) (SweepResult :type Hit%20Result%20Structure%20%28by%20ref%29))
  (if (not (Variables|Default|GetbIsMoving))
    (Utilities|FlowControl|Delay 0.4)
    (CallFunction|AnimCode)))

(event Custom|AnimCode
  (Variables|Default|SetbIsMoving true)
  (bind (_direction _animpercedntage) (Timeline|PlatformAnim PlayFromStart)
    (:Update
      (Transformation|SetRelativeLocation (Variables|Default|GetCube) (Math|Vector|Lerp(Vector) "0, 0, 0" "0, 0,500.000000" _animpercedntage) false false))
    (:Finished
      (Utilities|FlowControl|Delay 1.0)
      (if (Utilities|Enum|Equal(Enum) _direction "Forward")
        (Components|Timeline|ReversefromEnd (Variables|Default|GetPlatformAnim))
        (else
          (Variables|Default|SetbIsMoving false))))))

(event EventBeginPlay)

(fn ConstructionScript)