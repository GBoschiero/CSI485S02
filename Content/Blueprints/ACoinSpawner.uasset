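; Coin spawner actor that places an ACoin at its Billboard's transform when play begins.
; Each coin receives a randomly selected score from four fixed values and a reference back to this spawner.
; A Respawn event spawns a new coin after a short delay.
; A debug print shows a random score, but its separate random roll means it can differ from the coin's actual score.
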(event Custom|SpawnCoin
  (bind _returnvalue (Math|Random|RandomIntegerinRange 0 3))
  (bind _returnvalue_2 (Utilities|Select :Index _returnvalue :Option%200 50 :Option%201 100 :Option%202 250 :Option%203 500))
  (Development|PrintString (Utilities|String|ToString(Integer) _returnvalue_2) true true "(R=1.000000,G=0.000000,B=0.040900,A=1.000000)" 1e+01)
  (Game|SpawnActorfromClass "/Game/Blueprints/ACoin.ACoin_C" (Transformation|GetWorldTransform (Variables|Default|GetBillboard)) "Undefined" 0 self _returnvalue_2 0))

(event Custom|Respawn
  (Utilities|FlowControl|Delay 2.0)
  (CallFunction|SpawnCoin))

(event EventBeginPlay
  (CallFunction|SpawnCoin))

(fn ConstructionScript)